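; Gameplay ability that performs a dash along the avatar's current horizontal velocity.
; On activation it commits the ability or cancels, then starts a montage task and immediately applies a short constant root motion force.
; Direction is normalized XY velocity, so a stationary avatar gets a zero vector.
; The ability ends when the force finishes, independent of montage completion, keeping the last root motion velocity.
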(event `self.K2_ActivateAbility`
  (bind _returnvalue (`self.K2_CommitAbility`))
  (if _returnvalue
    (`AbilityTask_PlayMontageAndWait.CreatePlayMontageAndWaitProxy` "None"
      (:`then`
        (`AbilityTask_ApplyRootMotionConstantForce.ApplyRootMotionConstantForce` "None" (`KismetMathLibrary.Normal` (`KismetMathLibrary.MakeVector` (.x (`Actor.GetVelocity` (`self.GetAvatarActorFromActorInfo`))) (.y (`Actor.GetVelocity` (`self.GetAvatarActorFromActorInfo`))))) 4000.0 0.3 false null "MaintainLastRootMotionVelocity"
          (:`OnFinish`
            (`self.K2_EndAbility`)))))
    (else
      (`self.K2_CancelAbility`))))