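; Gameplay Ability that makes the avatar jump along its facing direction using an ApplyRootMotionJumpForce task.
; Jump distance and height come from owner attributes, with separate picks based on whether the Character.Sprint tag is present.
; Distance drops to zero when the avatar has no velocity, giving a jump in place.
; The jump keeps its last root motion velocity on finish, and the ability ends on finish or landing.
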(event `self.K2_ActivateAbility`
  (bind ((`OwnerActor` _owneractor)) (break `GameplayAbilityActorInfo` (`self.L_ActorInfo`)))
  (bind ((`OwnerActor` _owneractor_2) (`AvatarActor` _avataractor)) (break `GameplayAbilityActorInfo` (`self.L_ActorInfo`)))
  (set `self.L_ActorInfo` (`self.GetActorInfo`))
  (bind _returnvalue (message `GameplayTagAssetInterface.HasMatchingGameplayTag` (`.AbilitySystemComponent` (break `GameplayAbilityActorInfo` (`self.L_ActorInfo`))) (struct :`TagName` "Character.Sprint")))
  (set `self.L_HasSprintTag` _returnvalue)
  (`AbilityTask_ApplyRootMotionJumpForce.ApplyRootMotionJumpForce` "None" (`Actor.K2_GetActorRotation` (`.AvatarActor` (break `GameplayAbilityActorInfo` (`self.L_ActorInfo`)))) (`KismetMathLibrary.SelectFloat` (`KismetMathLibrary.SelectFloat` (`.ReturnValue` (`AbilitySystemBlueprintLibrary.GetFloatAttribute` _owneractor_2 (struct :`AttributeName` "BoostJumpLength" :`Attribute` "/Script/SecretTemple.STAttributeSet:BoostJumpLength" :`AttributeOwner` "Class'\"/Script/SecretTemple.STAttributeSet\"'"))) (`.ReturnValue` (`AbilitySystemBlueprintLibrary.GetFloatAttribute` _owneractor_2 (struct :`AttributeName` "StandardJumpLength" :`Attribute` "/Script/SecretTemple.STAttributeSet:StandardJumpLength" :`AttributeOwner` "Class'\"/Script/SecretTemple.STAttributeSet\"'"))) (`self.L_HasSprintTag`)) 0.0 (> (`KismetMathLibrary.VSize` (`Actor.GetVelocity` _avataractor)) 0.0)) (`KismetMathLibrary.SelectFloat` (`.ReturnValue` (`AbilitySystemBlueprintLibrary.GetFloatAttribute` _owneractor (struct :`AttributeName` "BoostJumpHeight" :`Attribute` "/Script/SecretTemple.STAttributeSet:BoostJumpHeight" :`AttributeOwner` "Class'\"/Script/SecretTemple.STAttributeSet\"'"))) (`.ReturnValue` (`AbilitySystemBlueprintLibrary.GetFloatAttribute` _owneractor (struct :`AttributeName` "StandardJumpHeight" :`Attribute` "/Script/SecretTemple.STAttributeSet:StandardJumpHeight" :`AttributeOwner` "Class'\"/Script/SecretTemple.STAttributeSet\"'"))) (`self.L_HasSprintTag`)) 0.75 0.75 false "MaintainLastRootMotionVelocity"
    (:`OnFinish`
      _)
    (:`OnLanded`
      _))
  (`self.K2_EndAbility`))