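; Projectile actor for the gun ability that damages characters through the Gameplay Ability System.
; Its lifespan is derived from range and initial speed, so it expires at maximum range.
; On overlapping a non-instigator Character with an ability system, it runs a zero-length pawn trace to recover a hit result for that target.
; It adds that hit to the damage spec's effect context, applies the spec and destroys itself.
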(event `self.ReceiveBeginPlay`
  (`self.SetLifeSpan` (/ (`self.Range`) (`ProjectileMovementComponent.InitialSpeed` (`self.ProjectileMovement`)))))

(event `self.Collision.OnComponentBeginOverlap`
  (params (OverlappedComponent :type "PrimitiveComponent Object Reference") (OtherActor :type "Actor Object Reference") (OtherComp :type "PrimitiveComponent Object Reference") (OtherBodyIndex :type Integer) (bFromSweep :type Boolean) (SweepResult :type "HitResult Structure (by ref)"))
  (if (!= OtherActor (`self.GetInstigator`))
    (bind _ascharacter (cast `Character` OtherActor))
    (bind _returnvalue (`AbilitySystemBlueprintLibrary.GetAbilitySystemComponent` _ascharacter))
    (`/Engine/EditorBlueprintResources/StandardMacros.IsValid` _returnvalue
      (:`Is Valid`
        (bind _outhits (`KismetSystemLibrary.LineTraceMultiForObjects` :`Start` (`self.K2_GetActorLocation`) :`End` (`self.K2_GetActorLocation`) :`ObjectTypes` (`|MakeArray` "ObjectTypeQuery3" :!type "EObjectTypeQuery Enum") :`DrawTime` 2.0))
        (for _array_element _outhits
          (if (== (`.HitActor` (`GameplayStatics.BreakHitResult` _array_element)) _ascharacter)
            (set `self.FinalHit` _array_element)
            (break)))
        (bind _returnvalue_2 (`AbilitySystemBlueprintLibrary.GetEffectContext` (`self.DamageEffectSpecHandle`)))
        (`AbilitySystemBlueprintLibrary.EffectContextAddHitResult` _returnvalue_2 (`self.FinalHit`))
        (`AbilitySystemComponent.BP_ApplyGameplayEffectSpecToSelf` _returnvalue (`self.DamageEffectSpecHandle`))
        (`self.K2_DestroyActor`)))))

(event `self.SM_Body.OnComponentBeginOverlap`
  (params (OverlappedComponent :type "PrimitiveComponent Object Reference") (OtherActor :type "Actor Object Reference") (OtherComp :type "PrimitiveComponent Object Reference") (OtherBodyIndex :type Integer) (bFromSweep :type Boolean) (SweepResult :type "HitResult Structure (by ref)")))

(fn `UserConstructionScript`)