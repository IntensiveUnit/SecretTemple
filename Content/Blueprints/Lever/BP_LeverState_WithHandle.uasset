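; Lever state for a BP_Lever with its handle attached, showing the handle mesh and handling interaction while no handle animation plays.
; Interacting toggles the owner's WasActivated flag, fires a try-activate or try-deactivate event, then waits for a response.
; Approval plays the pull timeline forward or in reverse and fires the confirming event, while refusal restores the flag and plays a shake.
; Both timelines lerp the handle pivot between start and end transforms.
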(fn `CanInteractWithActor`
  (params (InteractionInstigator :type "PlayerCharacter Object Reference"))
  (returns (ReturnValue :type Boolean))
  (return (and (not (`TimelineComponent.IsPlaying` (`self.PullLeverHandle`))) (not (`TimelineComponent.IsPlaying` (`self.ShakeLeverHandle`))))))

(fn `InteractWithActor`
  (params (InteractionInstigator :type "PlayerCharacter Object Reference"))
  (returns (ReturnValue :type Boolean))
  (bind _asbp_lever (cast `/Game/Blueprints/Lever/BP_Lever` (`self.GetOwner`)))
  (bind _output_get (set `/Game/Blueprints/Lever/BP_Lever.bWasActivated` (not (`/Game/Blueprints/Lever/BP_Lever.bWasActivated` _asbp_lever)) _asbp_lever))
  (if _output_get
    (`/Game/Blueprints/Lever/BP_Lever.OnTryToActivate` _asbp_lever _asbp_lever)
    (else
      (`/Game/Blueprints/Lever/BP_Lever.OnTryToDeactivate` _asbp_lever _asbp_lever)))
  (return true) ; Waiting for response
)

(fn `TakeResponseFromActor`
  (params (ResponseInstigator :type "Actor Object Reference") (bResponse :type Boolean :default false))
  (returns (ReturnValue :type Boolean))
  (if bResponse
    (bind _asbp_lever (cast `/Game/Blueprints/Lever/BP_Lever` (`self.GetOwner`)))
    (if (`/Game/Blueprints/Lever/BP_Lever.bWasActivated` _asbp_lever)
      (`TimelineComponent.PlayFromStart` (`self.PullLeverHandle`))
      (`/Game/Blueprints/Lever/BP_Lever.OnActivated` _asbp_lever _asbp_lever)
      (return false)
      (else
        (`TimelineComponent.ReverseFromEnd` (`self.PullLeverHandle`))
        (`/Game/Blueprints/Lever/BP_Lever.OnDeactivated` _asbp_lever _asbp_lever)
        (return false)))
    (else
      (bind _asbp_lever_2 (cast `/Game/Blueprints/Lever/BP_Lever` (`self.GetOwner`)))
      (set `/Game/Blueprints/Lever/BP_Lever.bWasActivated` (not (`/Game/Blueprints/Lever/BP_Lever.bWasActivated` _asbp_lever_2)) _asbp_lever_2) ; Restore previous WasActivated
      (`TimelineComponent.PlayFromStart` (`self.ShakeLeverHandle`))
      (return false))))

(fn `UserConstructionScript`
  (bind _asbp_lever (cast `/Game/Blueprints/Lever/BP_Lever` (`self.GetOwner`)))
  (`SceneComponent.SetVisibility` (`/Game/Blueprints/Lever/BP_Lever.SM_Handle` _asbp_lever) true false))