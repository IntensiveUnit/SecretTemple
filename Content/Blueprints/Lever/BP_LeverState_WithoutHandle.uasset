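; State object for BP_Lever while its handle is missing, letting the player fit one from the inventory.
; Interacting blends the view to the lever and opens the HUD's inventory menu.
; Using a BP_LeverHandle removes and destroys the item, reveals the handle mesh and plays a timeline moving its pivot into place.
; When the timeline finishes, it restores the player's view, closes the menu and switches the lever's state.
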(event `PlayAnimation`
  (bind _asbp_lever (cast `/Game/Blueprints/Lever/BP_Lever` (`self.GetOwner`)))
  (bind (_direction _animation) (`Timeline|HandleAddedAnimation` :!via `PlayFromStart`)
    (:`Update`
      (`SceneComponent.K2_SetRelativeLocationAndRotation` (`/Game/Blueprints/Lever/BP_Lever.SC_HandlePivot` _asbp_lever) (`KismetMathLibrary.VLerp` (.location (`self.StartAnimationTransform`)) (.location (`self.EndAnimationTransform`)) _animation) (`KismetMathLibrary.RLerp` (.rotation (`self.StartAnimationTransform`)) (.rotation (`self.EndAnimationTransform`)) _animation) false false))
    (:`Finished`
      (`self.OnInteractionInterrupted`)
      (bind _asbp_lever_2 (cast `/Game/Blueprints/Lever/BP_Lever` (`self.GetOwner`)))
      (`/Game/Blueprints/Lever/BP_Lever.SetCurrentState` _asbp_lever_2 "NewEnumerator1"))))

(fn `CanInteractWithActor`
  (params (InteractionInstigator :type "PlayerCharacter Object Reference"))
  (returns (ReturnValue :type Boolean))
  (return true))

(fn `InteractWithActor`
  (params (InteractionInstigator :type "PlayerCharacter Object Reference"))
  (returns (ReturnValue :type Boolean))
  (locals (L_InteractingPlayerCharacter :type "PlayerCharacter Object Reference") (L_InteractingActorHUD :type "/Game/Blueprints/GameplayFramework/BP_HUD Object Reference"))
  (bind _asbp_player_controller (cast `/Game/Blueprints/GameplayFramework/BP_PlayerController` (`Pawn.GetController` InteractionInstigator)))
  (set `self.InteractingPlayerController` _asbp_player_controller)
  (bind _asplayer_character (cast `PlayerCharacter` (`Controller.K2_GetPawn` (`self.InteractingPlayerController`))))
  (bind _output_get (set `local.L_InteractingPlayerCharacter` _asplayer_character))
  (add `PlayerCharacter.OnInteractionInterrupted` _output_get (`|CreateDelegate` :!event `OnInteractionInterrupted`))
  (`PlayerController.SetViewTargetWithBlend` (`self.InteractingPlayerController`) (`self.GetOwner`) 0.0 "VTBlend_PreBlended" 0.0 false)
  (`PlayerCharacter.SetIsCharacterInteracts` (`local.L_InteractingPlayerCharacter`) (`self.GetOwner`))
  (bind _asbp_hud (cast `/Game/Blueprints/GameplayFramework/BP_HUD` (`PlayerController.GetHUD` (`self.InteractingPlayerController`))))
  (set `local.L_InteractingActorHUD` _asbp_hud)
  (`/Game/Blueprints/GameplayFramework/BP_HUD.OpenInteractiveMenu` (`local.L_InteractingActorHUD`) (`PlayerCharacter.GetInventoryComponent` (`local.L_InteractingPlayerCharacter`)) self)
  (return true))

(fn `OnInteractionInterrupted`
  (bind _interactingplayercontroller (`self.InteractingPlayerController`))
  (`self.InteractingPlayerController`
    (:`then`
      (`PlayerController.SetViewTargetWithBlend` _interactingplayercontroller (`Controller.K2_GetPawn` _interactingplayercontroller) 0.0 "VTBlend_PreBlended" 0.0 false)
      (bind _asplayer_character (cast `PlayerCharacter` (`Controller.K2_GetPawn` (`self.InteractingPlayerController`))))
      (`PlayerCharacter.SetIsCharacterInteracts` _asplayer_character null)
      (bind _asbp_player_controller (cast `/Game/Blueprints/GameplayFramework/BP_PlayerController` (`self.InteractingPlayerController`)))
      (bind _asbp_hud (cast `/Game/Blueprints/GameplayFramework/BP_HUD` (`PlayerController.GetHUD` _asbp_player_controller)))
      (`/Game/Blueprints/GameplayFramework/BP_HUD.CloseInteractionMenu` _asbp_hud)
      (set `self.InteractingPlayerController` null)
      (return))
    (:`else`)))

(fn `UseItemOnActor`
  (params (InteractionInstigator :type "PlayerCharacter Object Reference") (Item :type "Item Object Reference"))
  (returns (ReturnValue :type Boolean))
  (locals (L_InteractingInstigator :type "PlayerCharacter Object Reference") (L_LeverHandle :type "/Game/Blueprints/Items/Collectibles/BP_LeverHandle Object Reference"))
  (set `local.L_InteractingInstigator` InteractionInstigator)
  (bind _asbp_lever_handle (cast `/Game/Blueprints/Items/Collectibles/BP_LeverHandle` Item)
    (:`then`
      (bind _output_get (set `local.L_LeverHandle` _asbp_lever_handle))
      (bind _returnvalue (`InventoryComponent.RemoveCollectibleItem` (`PlayerCharacter.GetInventoryComponent` (`local.L_InteractingInstigator`)) _output_get))
      (if _returnvalue
        (bind _asbp_lever (cast `/Game/Blueprints/Lever/BP_Lever` (`self.GetOwner`))
          (:`then`
            (`SceneComponent.SetVisibility` (`/Game/Blueprints/Lever/BP_Lever.SM_Handle` _asbp_lever) true false)
            (`self.PlayAnimation`)
            (`self.K2_DestroyActor` (`local.L_LeverHandle`))
            (return false))
          (:`CastFailed`
            (return false)))
        (else
          (return false))))
    (:`CastFailed`
      (return false))))

(fn `UserConstructionScript`)