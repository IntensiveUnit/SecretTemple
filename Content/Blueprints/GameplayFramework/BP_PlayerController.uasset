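; Player controller that opens the inventory and switches input between gameplay and UI.
; The Inventory input action casts the HUD to BP_HUD and calls its OpenInventory.
; SetPlayerInputMode toggles cursor visibility, blocks or restores look and move input, and sets either Game-and-UI mode focused on a given widget or Game Only mode.
; It resets the ignore-input flags before setting them, so repeated calls do not stack.
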(event `InputAction|Inventory`
  (params (Key :type "Key Structure"))
  (:`Pressed`
    (bind _asbp_hud (cast `/Game/Blueprints/GameplayFramework/BP_HUD` (`self.GetHUD`)))
    (`/Game/Blueprints/GameplayFramework/BP_HUD.OpenInventory` _asbp_hud)))

(fn `SetPlayerInputMode`
  (params (bIsUIMode :type Boolean) (InWidgetToFocus :type "Widget Object Reference"))
  ;[1 1 1] Use this function to toggle between UI mode and Game mode when display user interface to the player
  ; when you display UI in the screen and you need mouse cursor to show up call this function and set UI mode to ture
  ; Otherwise set UI mode to false
  (set `self.bShowMouseCursor` bIsUIMode)
  (`self.ResetIgnoreLookInput`)
  (`self.SetIgnoreLookInput` bIsUIMode)
  (`self.ResetIgnoreMoveInput`)
  (`self.SetIgnoreMoveInput` bIsUIMode)
  (if bIsUIMode
    (`WidgetBlueprintLibrary.SetInputMode_GameAndUIEx` self InWidgetToFocus "DoNotLock" false)
    (else
      (`WidgetBlueprintLibrary.SetInputMode_GameOnly` self))))

(fn `UserConstructionScript`)