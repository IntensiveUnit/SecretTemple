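; Base actor implementing a state pattern, with lever states With Handle and Without Handle as separate spawned actors.
; InitializeState spawns the state at BeginPlay, but its switch is fixed to Without Handle and CurrentState is set to None, not the spawned actor.
; SetCurrentState updates the enum on change, then calls DestroyCurrentState and InitializeState.
; GetCurrentState re-initializes when the reference is invalid, and Destroyed calls DestroyCurrentState.
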(event `self.ReceiveBeginPlay`
  (`self.InitializeState`))

(event `self.ReceiveDestroyed`
  (`self.DestroyCurrentState`))

(fn `DestroyCurrentState`
  (`/Engine/EditorBlueprintResources/StandardMacros.IsValid` (`self.CurrentState`)
    (:`Is Valid`
      (`self.K2_DestroyActor` (`self.CurrentState`)))
    (:`Is Not Valid`
      _))
  (return))

(fn `GetCurrentState`
  (returns (CurrentState :type "/Game/Blueprints/StateSystem/States/BP_State Object Reference"))
  (`/Engine/EditorBlueprintResources/StandardMacros.IsValid` (`self.CurrentState`)
    (:`Is Valid`
      (return (`self.CurrentState`)))
    (:`Is Not Valid`
      (`self.InitializeState`)
      (return (`self.CurrentState`)))))

(fn `InitializeState`
  (switch `/Game/Blueprints/Lever/E_LeverStates` "NewEnumerator0"
    (:`NewEnumerator0`
      (`|SpawnActorFromClass` "/Game/Blueprints/Lever/BP_LeverState_WithoutHandle.BP_LeverState_WithoutHandle_C" (`self.GetTransform`) "Undefined" "OverrideRootScale" self null)
      (set `self.CurrentState` null)
      (return))
    (:`NewEnumerator1`
      (`|SpawnActorFromClass` "/Game/Blueprints/Lever/BP_LeverState_WithHandle.BP_LeverState_WithHandle_C" (`self.GetTransform`) "Undefined" "OverrideRootScale" self null)
      (set `self.CurrentState` null)
      (return))))

(fn `SetCurrentState`
  (params (InState :type "/Game/Blueprints/StateSystem/E_States Enum" :default "E_States_MAX"))
  (locals (L_NewState :type "/Game/Blueprints/StateSystem/E_States Enum"))
  (set `local.L_NewState` InState)
  (if (`|EnumInequality` (`local.L_NewState`) (`self.CurrentState_Enum`))
    (set `self.CurrentState_Enum` (`local.L_NewState`))
    (`self.DestroyCurrentState`)
    (`self.InitializeState`)
    (else
      (return))))

(fn `UserConstructionScript`)