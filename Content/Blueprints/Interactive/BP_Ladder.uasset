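; BP_Ladder is a parametric climbable ladder that gives the player a climbing ability through the Gameplay Ability System.
; The construction script sizes and offsets a trigger box from the ladder's depth, width and height, then stacks mesh segments at fixed intervals up the height.
; When a PlayerCharacter enters the box, GA_Climbing_BP is granted and activated once, and leaving clears it through the stored spec handle.
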(event `self.Box.OnComponentBeginOverlap`
  (params (OverlappedComponent :type "PrimitiveComponent Object Reference") (OtherActor :type "Actor Object Reference") (OtherComp :type "PrimitiveComponent Object Reference") (OtherBodyIndex :type Integer) (bFromSweep :type Boolean) (SweepResult :type "HitResult Structure (by ref)"))
  (bind _asplayer_character (cast `PlayerCharacter` OtherActor))
  (bind _returnvalue (`AbilitySystemComponent.K2_GiveAbilityAndActivateOnce` (`PlayerCharacter.GetAbilitySystemComponent` _asplayer_character) "/Game/GameplayAbility/Climbing/GA_Climbing_BP.GA_Climbing_BP_C" 0 -1))
  (set `self.GameplayAbilitySpecHandle` _returnvalue))

(event `self.Box.OnComponentEndOverlap`
  (params (OverlappedComponent :type "PrimitiveComponent Object Reference") (OtherActor :type "Actor Object Reference") (OtherComp :type "PrimitiveComponent Object Reference") (OtherBodyIndex :type Integer))
  (bind _asplayer_character (cast `PlayerCharacter` OtherActor))
  (`AbilitySystemComponent.ClearAbility` (`PlayerCharacter.GetAbilitySystemComponent` _asplayer_character) (`self.GameplayAbilitySpecHandle`)))

(fn `UserConstructionScript`
  (bind _returnvalue (/ (`self.LadderHeight`) 2.0))
  (`BoxComponent.SetBoxExtent` (`self.Box`) (`KismetMathLibrary.MakeVector` (`self.LadderDepth`) (`self.LadderWidth`) _returnvalue) true)
  (`SceneComponent.K2_AddRelativeLocation` (`self.Box`) (`KismetMathLibrary.MakeVector` (/ (`self.LadderDepth`) 2.0) 0.0 _returnvalue) false true)
  (for _index (range (`KismetMathLibrary.FTrunc` (/ (`self.LadderHeight`) 35.0)))
    (bind _returnvalue_2 (`AddComponent|NODE_AddStaticMeshComponent-2` :`RelativeTransform` (`KismetMathLibrary.MakeTransform` (`KismetMathLibrary.MakeVector` 0.0 0.0 (* _index 35.0)))))
    (`StaticMeshComponent.SetStaticMesh` _returnvalue_2 (`self.SM_Ladder`))))