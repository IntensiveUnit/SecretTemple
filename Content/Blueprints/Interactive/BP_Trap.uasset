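; Interactive spike trap that, when activated, turns red as a warning and fires its spikes after a short delay.
; A timeline lerps the spikes out, then reverses to retract them, restore the material and call OnDeactivated.
; Once the spikes emerge, player characters overlapping the box receive a GAS damage effect through their PlayerState.
; A DamageDone flag limits damage to one pass and is never reset here.
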(event `Activate`
  (if (not (`self.IsPlaying`))
    (`PrimitiveComponent.SetMaterial` (`self.SM_Trap`) 1 "/AnimationSharing/AnimSharingRed.AnimSharingRed")
    (set `self.IsPlaying` true)
    (`KismetSystemLibrary.Delay` 3.0)
    (bind (_direction _alpha) (`Timeline|Animation` :!via `PlayFromStart` :!label _label)
      (:`Update`
        (set `self.Alpha` _alpha)
        (`|ExecutionSequence`
          (:`then_0`
            (`SceneComponent.K2_SetRelativeLocation` (`self.SM_Spikes`) (`KismetMathLibrary.VLerp` (`self.InitialLocation`) (`self.EndLocation`) (`self.Alpha`)) false false))
          (:`then_1`
            (if (and (not (`self.DamageDone`)) (> (`self.Alpha`) 0.2))
              (for _array_element (`PrimitiveComponent.GetOverlappingActors` (`self.Box`) "/Script/SecretTemple.PlayerCharacter")
                (bind _asplayer_character (cast `PlayerCharacter` _array_element))
                (`/Engine/EditorBlueprintResources/StandardMacros.IsValid` _asplayer_character
                  (:`Is Valid`
                    (set `self.DamageDone` true)
                    (bind _returnvalue (`AbilitySystemBlueprintLibrary.GetAbilitySystemComponent` (`Pawn.PlayerState` _asplayer_character)))
                    (`AbilitySystemComponent.BP_ApplyGameplayEffectToTarget` :`self` _returnvalue :`GameplayEffectClass` "/Game/Abilities/GameplayEffects/GE_Damage_BP.GE_Damage_BP_C" :`Target` _returnvalue))))))))
      (:`Finished`
        (switch `ETimelineDirection` _direction
          (:`Forward`
            (`self.ReverseAnimation`))
          (:`Backward`
            (`self.Deactivate`)))))))

(event `ReverseAnimation`
  (goto _label :!via `ReverseFromEnd`))

(fn `Deactivate`
  (set `self.IsPlaying` false)
  (`PrimitiveComponent.SetMaterial` (`self.SM_Trap`) 1 "/Game/secretttemple/Meshes/Building/Armory/Materials/Material_003.Material_003")
  (`self.OnDeactivated` self))

(fn `UserConstructionScript`)