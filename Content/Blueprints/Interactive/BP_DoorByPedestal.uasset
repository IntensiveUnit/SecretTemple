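; Door actor that opens by playing a level sequence once all of its linked pedestals are activated.
; On BeginPlay it binds to each pedestal's activate and deactivate events and keeps a count of active ones.
; Any deactivation lowers the count and reverses the sequence, but only if the player is currently paused.
; The construction script holds only disconnected editor-visualization experiments with arrows, index labels and widgets toward pedestals.
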(event `OpenDoor`
  (`self.LevelSequence`
    (:`then`
      (`MovieSceneSequencePlayer.Play` (`LevelSequenceActor.SequencePlayer` (`self.LevelSequence`))))
    (:`else`)))

(event `CloseDoor`
  (`self.LevelSequence`
    (:`then`
      (if (`MovieSceneSequencePlayer.IsPaused` (`LevelSequenceActor.SequencePlayer` (`self.LevelSequence`)))
        (`MovieSceneSequencePlayer.PlayReverse` (`LevelSequenceActor.SequencePlayer` (`self.LevelSequence`)))))
    (:`else`)))

(event `self.ReceiveBeginPlay`
  (for _array_element (`self.Pedestals`)
    (add `/Game/Blueprints/Interactive/BP_Pedestal.PedestalActivated` _array_element (delegate `PedestalActivated`))
    (add `/Game/Blueprints/Interactive/BP_Pedestal.PedestalDeactivated` _array_element (delegate `PedestalDeactivated`))))

(event `PedestalActivated`
  (params (InPedestal :type "/Game/Blueprints/Interactive/BP_Pedestal Object Reference"))
  (`/Engine/EditorBlueprintResources/StandardMacros.IncrementInt` (`self.ActivatedPedestalsNum`)
    (:`  `
      (if (>= (`self.ActivatedPedestalsNum`) (`KismetArrayLibrary.Array_Length` (`self.Pedestals`)))
        (`self.OpenDoor`)))))

(event `PedestalDeactivated`
  (params (InPedestal :type "/Game/Blueprints/Interactive/BP_Pedestal Object Reference"))
  (`/Engine/EditorBlueprintResources/StandardMacros.DecrementInt` (`self.ActivatedPedestalsNum`)
    (:`  `
      (`self.CloseDoor`))))

(fn `UserConstructionScript`)