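; Interactable gateway actor with a pivoting door and a separate barricade mesh.
; Interacting while closed calls OpenDoor, which swings the pivot via a timeline in a direction-selected way, then sets IsOpened and calls GateWayWasOpened; item use is refused.
; DestroyBarricade rotates the barricade and clears Barricaded, which interaction never checks.
; CloseDoor is empty, with its closing animation left unwired, as is the barricade visibility setup.
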(event `DestroyBarricade`
  (bind (_direction _alpha) (`Timeline|Animation_03` :!via `PlayFromStart`)
    (:`Update`
      (`SceneComponent.K2_SetRelativeRotation` (`self.SM_Barricade_01`) (`KismetMathLibrary.RLerp` (struct) (struct :`Pitch` 90.0) _alpha true) false false))
    (:`Finished`
      (set `self.Barricaded` false))))

(event `CloseDoor`)

(event `OpenDoor`
  (params (Direction :type Boolean))
  (bind (_direction _alpha) (`Timeline|Animation` :!via `PlayFromStart`)
    (:`Update`
      (`SceneComponent.K2_SetRelativeRotation` (`self.SC_Pivot_Door`) (`KismetMathLibrary.RLerp` (struct) (`KismetMathLibrary.SelectRotator` (struct :`Yaw` -90.0) (struct :`Yaw` 90.0) Direction) _alpha true) false false))
    (:`Finished`
      (set `self.IsOpened` true)
      (`self.GateWayWasOpened`))))

(fn `CanInteractWithActor`
  (params (InteractionInstigator :type "PlayerCharacter Object Reference"))
  (returns (ReturnValue :type Boolean))
  (return true))

(fn `CanUseItemOnActor`
  (params (InteractionInstigator :type "PlayerCharacter Object Reference") (Item :type "Item Object Reference"))
  (returns (ReturnValue :type Boolean))
  (return false))

(fn `InteractWithActor`
  (params (InteractionInstigator :type "PlayerCharacter Object Reference"))
  (returns (ReturnValue :type Boolean))
  (if (not (`self.IsOpened`))
    (`self.OpenDoor` false)
    (return true)))

(fn `UseItemOnActor`
  (params (InteractionInstigator :type "PlayerCharacter Object Reference") (Item :type "Item Object Reference"))
  (returns (ReturnValue :type Boolean))
  (return false))

(fn `UserConstructionScript`)