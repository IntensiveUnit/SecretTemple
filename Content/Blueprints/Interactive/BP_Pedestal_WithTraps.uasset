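; Interactive pedestal that springs a trap sequence when its item is picked up, unless a key was applied first.
; Pickup closes the door, plays a barricade sequence and activates a percentage-based number of randomly picked traps inside its box.
; A trap's deactivation chains further cycles until the count runs out, reversing the barricade.
; Interaction switches camera and opens an inventory menu, where the trap-room key can be used.
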(event `self.ReceiveBeginPlay`
  (add `CollectibleItem.OnCollectibleItemPickuped` (`self.TrapItem`) (delegate `OnTrapItemPickuped`)))

(event `OnTrapItemPickuped`
  (params (InItem :type "CollectibleItem Object Reference"))
  (if (not (`self.WasKeyApplied`))
    (set `self.bCanInteractWithActor` false)
    (set `/Game/Blueprints/Interactive/BP_Door.DoorLocked` true (`self.Door`))
    (`MovieSceneSequencePlayer.Play` (`LevelSequenceActor.SequencePlayer` (`self.BarricadeAnimation`)))
    (`/Game/Blueprints/Interactive/BP_Door.CloseDoor` (`self.Door`))
    (set `self.AmountOfTrapsToActivate` (`KismetMathLibrary.FCeil` (* (`KismetArrayLibrary.Array_Length` (`PrimitiveComponent.GetOverlappingActors` (`self.Box`) (`self.TrapClass`))) (`self.PercentageOfUsedTraps`))))
    (for _index (range (+ (`self.AmountOfTrapsToActivate`) 1)) :!label _label
      (bind _asbp_trap (cast `/Game/Blueprints/Interactive/BP_Trap` (`KismetArrayLibrary.Array_Random` (`PrimitiveComponent.GetOverlappingActors` (`self.Box`) (`self.TrapClass`)))))
      (`/Game/Blueprints/Interactive/BP_Trap.Activate` _asbp_trap)
      (if (== (`self.AmountOfTrapsToActivate`) _index)
        (add `/Game/Blueprints/Interactive/BP_Trap.OnDeactivated` _asbp_trap (delegate `ActivateAgain`))))
    (set `self.bCanInteractWithActor` true)
    (set `/Game/Blueprints/Interactive/BP_Door.DoorLocked` false (`self.Door`))))

(event `ActivateAgain`
  (params (Trap :type "/Game/Blueprints/Interactive/BP_Trap Object Reference"))
  (remove `/Game/Blueprints/Interactive/BP_Trap.OnDeactivated` Trap (delegate `ActivateAgain`))
  (bind _result (`/Engine/EditorBlueprintResources/StandardMacros.DecrementInt` (`self.TrapCycles`))
    (:`  `
      (if (> _result 0)
        (goto _label)
        (else
          (`MovieSceneSequencePlayer.PlayReverse` (`LevelSequenceActor.SequencePlayer` (`self.BarricadeAnimation`))))))))

(fn `CanInteractWithActor`
  (params (InteractionInstigator :type "PlayerCharacter Object Reference"))
  (returns (ReturnValue :type Boolean))
  (return (`self.bCanInteractWithActor`)))

(fn `InteractWithActor`
  (params (InteractionInstigator :type "PlayerCharacter Object Reference"))
  (returns (ReturnValue :type Boolean))
  (locals (L_PlayerCharacter :type "/Game/Characters/Mannequin/BP_PlayerCharacter Object Reference"))
  (bind _asbp_player_controller (cast `/Game/Blueprints/GameplayFramework/BP_PlayerController` (`Pawn.GetController` InteractionInstigator)))
  (set `self.OwnerController` _asbp_player_controller)
  (`self.OwnerController`
    (:`then`
      (bind _asbp_player_character (cast `/Game/Characters/Mannequin/BP_PlayerCharacter` (`Controller.K2_GetPawn` (`self.OwnerController`))))
      (bind _output_get (set `local.L_PlayerCharacter` _asbp_player_character))
      (add `PlayerCharacter.OnInteractionInterrupted` _output_get (`|CreateDelegate` :!event `OnInteractionInterrupted`))
      (`PlayerController.SetViewTargetWithBlend` (`self.OwnerController`) self 0.0 "VTBlend_PreBlended" 0.0 false)
      (`PlayerCharacter.SetIsCharacterInteracts` (`local.L_PlayerCharacter`) self)
      (bind _asbp_hud (cast `/Game/Blueprints/GameplayFramework/BP_HUD` (`PlayerController.GetHUD` (`self.OwnerController`))))
      (`/Game/Blueprints/GameplayFramework/BP_HUD.OpenInteractiveMenu` _asbp_hud (`PlayerCharacter.GetInventory` (`local.L_PlayerCharacter`)) self))
    (:`else`
      _))
  (for _array_element (`PrimitiveComponent.GetOverlappingActors` (`self.Sphere`) "/Script/Engine.Character")
    (`self.SetActorHiddenInGame` _array_element false))
  (return true))

(fn `OnInteractionInterrupted`
  (bind _ownercontroller (`self.OwnerController`)
    (:`then`
      (`PlayerController.SetViewTargetWithBlend` _ownercontroller (`Controller.K2_GetPawn` _ownercontroller) 0.0 "VTBlend_PreBlended" 0.0 false)
      (bind _asbp_player_character (cast `/Game/Characters/Mannequin/BP_PlayerCharacter` (`Controller.K2_GetPawn` _ownercontroller)))
      (`PlayerCharacter.SetIsCharacterInteracts` _asbp_player_character null)
      (bind _asbp_player_controller (cast `/Game/Blueprints/GameplayFramework/BP_PlayerController` (`self.OwnerController`)))
      (bind _asbp_hud (cast `/Game/Blueprints/GameplayFramework/BP_HUD` (`PlayerController.GetHUD` _asbp_player_controller)))
      (`/Game/Blueprints/GameplayFramework/BP_HUD.CloseInteractionMenu` _asbp_hud)
      (set `self.OwnerController` null))
    (:`else`
      _))
  (for _array_element (`PrimitiveComponent.GetOverlappingActors` (`self.Sphere`) "/Script/Engine.Character")
    (`self.SetActorHiddenInGame` _array_element false))
  (return))

(fn `TakeResponseFromActor`
  (params (ResponseInstigator :type "Actor Object Reference") (bResponse :type Boolean))
  (returns (ReturnValue :type Boolean))
  (return false))

(fn `UseItemOnActor`
  (params (InteractionInstigator :type "PlayerCharacter Object Reference") (Item :type "Item Object Reference"))
  (returns (ReturnValue :type Boolean))
  (locals (L_InteractionInstigator :type "PlayerCharacter Object Reference") (L_Key :type "/Game/Blueprints/Items/Collectibles/BP_KeyForTrapRoom Object Reference") (L_WasRemoved :type Boolean :default false))
  (set `local.L_InteractionInstigator` InteractionInstigator)
  (bind _asbp_key_for_trap_room (cast `/Game/Blueprints/Items/Collectibles/BP_KeyForTrapRoom` Item)
    (:`then`
      (set `local.L_Key` _asbp_key_for_trap_room)
      (bind _returnvalue (`InventoryComponent.RemoveCollectibleItem` (`PlayerCharacter.InventoryComponent` (`local.L_InteractionInstigator`)) (`local.L_Key`)))
      (set `local.L_WasRemoved` _returnvalue)
      (if (`local.L_WasRemoved`)
        (set `/Game/Blueprints/Items/Collectibles/BP_KeyForTrapRoom.WasUsed` true (`local.L_Key`))
        (`self.K2_AttachToComponent` (`local.L_Key`) (`self.SC_ItemPivot`) "None" "SnapToTarget" "SnapToTarget" "SnapToTarget" true)
        (`TimelineComponent.Play` (`self.AnimationSucces`))
        (set `self.bCanInteractWithActor` false)
        (set `self.WasKeyApplied` true)
        (return true)
        (else
          (return false))))
    (:`CastFailed`
      (return true))))

(fn `UserConstructionScript`)