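; Interactive puzzle pedestal that accepts a Saint/Devil statuette and signals activation when its top and bottom sides match the pedestal's configured numbers.
; Interacting blends the view to the pedestal and opens the inventory menu until interrupted.
; Any such statuette attaches to the pivot with a sequence, which reverses on pickup alongside a deactivation signal; other items play a wrong-item sequence.
; Construction labels both sides and can preview animation endpoints.
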(event `OnItemPickedUp`
  (params (Item :type "Item Object Reference") (WhoPickedUp :type "PlayerCharacter Object Reference"))
  (message `/Game/Blueprints/Items/BPI_ItemInteraction.DetachFromComponent` Item)
  (`MovieSceneSequencePlayer.PlayReverse` (`ActorSequenceComponent.SequencePlayer` (`self.AS_RightItem`)))
  (`self.PedestalDeactivated` self))

(fn `CanInteractWithActor`
  (params (InteractionInstigator :type "PlayerCharacter Object Reference"))
  (returns (ReturnValue :type Boolean))
  (return true))

(fn `InteractWithActor`
  (params (InteractionInstigator :type "PlayerCharacter Object Reference"))
  (returns (ReturnValue :type Boolean))
  (locals (L_PlayerCharacter :type "PlayerCharacter Object Reference"))
  (bind _asbp_player_controller (cast `/Game/Blueprints/GameplayFramework/BP_PlayerController` (`Pawn.GetController` InteractionInstigator)))
  (set `self.OwnerController` _asbp_player_controller)
  (`self.OwnerController`
    (:`then`
      (bind _asplayer_character (cast `PlayerCharacter` (`Controller.K2_GetPawn` (`self.OwnerController`))))
      (bind _output_get (set `local.L_PlayerCharacter` _asplayer_character))
      (add `PlayerCharacter.OnInteractionInterrupted` _output_get (`|CreateDelegate` :!event `OnInteractionInterrupted`))
      (`PlayerController.SetViewTargetWithBlend` (`self.OwnerController`) self 0.0 "VTBlend_PreBlended" 0.0 false)
      (`PlayerCharacter.SetIsCharacterInteracts` (`local.L_PlayerCharacter`) self)
      (bind _asbp_hud (cast `/Game/Blueprints/GameplayFramework/BP_HUD` (`PlayerController.GetHUD` (`self.OwnerController`))))
      (`/Game/Blueprints/GameplayFramework/BP_HUD.OpenInteractiveMenu` _asbp_hud (`PlayerCharacter.GetInventoryComponent` (`local.L_PlayerCharacter`)) self))
    (:`else`
      _))
  (return true))

(fn `OnInteractionInterrupted`
  (bind _ownercontroller (`self.OwnerController`)
    (:`then`
      (`PlayerController.SetViewTargetWithBlend` _ownercontroller (`Controller.K2_GetPawn` _ownercontroller) 0.0 "VTBlend_PreBlended" 0.0 false)
      (bind _asplayer_character (cast `PlayerCharacter` (`Controller.K2_GetPawn` _ownercontroller)))
      (`PlayerCharacter.SetIsCharacterInteracts` _asplayer_character null)
      (bind _asbp_player_controller (cast `/Game/Blueprints/GameplayFramework/BP_PlayerController` (`self.OwnerController`)))
      (bind _asbp_hud (cast `/Game/Blueprints/GameplayFramework/BP_HUD` (`PlayerController.GetHUD` _asbp_player_controller)))
      (`/Game/Blueprints/GameplayFramework/BP_HUD.CloseInteractionMenu` _asbp_hud)
      (set `self.OwnerController` null))
    (:`else`
      _))
  (for _array_element (`PrimitiveComponent.GetOverlappingActors` (`self.Sphere`) "/Script/Engine.Character")
    (`self.SetActorHiddenInGame` _array_element false))
  (return))

(fn `StatuetteHasRightSides`
  (params (Statuette :type "/Game/Blueprints/Items/Collectibles/SaintAndDevilStatuette/BP_CollectibleItem_SaintDevil Object Reference"))
  (returns (ReturnValue :type Boolean))
  (return (and (`|EnumEquality` (`/Game/Blueprints/Items/Collectibles/SaintAndDevilStatuette/BP_CollectibleItem_SaintDevil.GetCurrentTopSide` Statuette) (`self.SaintSideNumber`)) (`|EnumEquality` (`/Game/Blueprints/Items/Collectibles/SaintAndDevilStatuette/BP_CollectibleItem_SaintDevil.GetCurrentBottomSide` Statuette) (`self.DevilSideNumber`)))))

(fn `UseItemOnActor`
  (params (InteractionInstigator :type "PlayerCharacter Object Reference") (Item :type "Item Object Reference"))
  (returns (ReturnValue :type Boolean))
  (locals (L_InteractionInstigator :type "PlayerCharacter Object Reference") (L_SaintDevilStatuette :type "/Game/Blueprints/Items/Collectibles/SaintAndDevilStatuette/BP_CollectibleItem_SaintDevil Object Reference"))
  (set `local.L_InteractionInstigator` InteractionInstigator)
  (bind _asbp_collectible_item_saint_devil (cast `/Game/Blueprints/Items/Collectibles/SaintAndDevilStatuette/BP_CollectibleItem_SaintDevil` Item)
    (:`then`
      (set `local.L_SaintDevilStatuette` _asbp_collectible_item_saint_devil)
      (bind _returnvalue (`InventoryComponent.RemoveCollectibleItem` (`PlayerCharacter.GetInventoryComponent` (`local.L_InteractionInstigator`)) (`local.L_SaintDevilStatuette`)))
      (if _returnvalue
        (message `/Game/Blueprints/Items/BPI_ItemInteraction.AttachToComponent` (`local.L_SaintDevilStatuette`) (`self.SC_Pivot`) false)
        (add `Item.OnItemWasPickedUp` (`local.L_SaintDevilStatuette`) (`|CreateDelegate` :!event `OnItemPickedUp`))
        (`MovieSceneSequencePlayer.Play` (`ActorSequenceComponent.SequencePlayer` (`self.AS_RightItem`)))
        (bind _returnvalue_2 (`self.StatuetteHasRightSides` (`local.L_SaintDevilStatuette`)))
        (if _returnvalue_2
          (`self.PedestalActivated` self)
          (return true)
          (else
            (return true)))
        (else
          (`MovieSceneSequencePlayer.Play` (`ActorSequenceComponent.SequencePlayer` (`self.AS_WrongItem`)))
          (return false))))
    (:`CastFailed`
      (`MovieSceneSequencePlayer.Play` (`ActorSequenceComponent.SequencePlayer` (`self.AS_WrongItem`)))
      (return false))))

(fn `UserConstructionScript`
  (`TextRenderComponent.K2_SetText` (`self.TextRender_DevilSide`) (`KismetTextLibrary.Conv_IntToText` (+ (`KismetMathLibrary.Conv_ByteToInt` (`self.DevilSideNumber`)) 1)))
  (`TextRenderComponent.K2_SetText` (`self.TextRender_SaintSide`) (`KismetTextLibrary.Conv_IntToText` (+ (`KismetMathLibrary.Conv_ByteToInt` (`self.SaintSideNumber`)) 1)))
  (if (`self.DebugAnimation`)
    (bind _returnvalue (`AddComponent|NODE_AddStaticMeshComponent-0`))
    (`SceneComponent.K2_SetRelativeTransform` _returnvalue (`self.StartAnimationTransform`) false true)
    (bind _returnvalue_2 (`AddComponent|NODE_AddStaticMeshComponent-1`))
    (`SceneComponent.K2_SetRelativeTransform` _returnvalue_2 (`self.EndAnimationTransform`) false true)))