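; Parent Blueprint for note items, providing attach, detach and snapshot-pivot functions for handling the note on other components.
; AttachToComponent caches both pivots' relative transforms, then snaps either the rotation or translation pivot onto the given component.
; DetachFromComponent detaches both pivots, reattaches the rotation pivot to root, restores cached transforms and parks the actor far below the world origin.
; Rotate is a stub returning false; event graph and construction script are empty.
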(fn `AttachToComponent`
  (params (Component :type "SceneComponent Object Reference") (ForRotation :type Boolean))
  (returns (ReturnValue :type Boolean))
  (locals (L_Component :type "SceneComponent Object Reference") (L_Rotation :type Boolean))
  (set `local.L_Component` Component)
  (set `local.L_Rotation` ForRotation)
  (set `self.CachedRotationPivotTransform` (`SceneComponent.GetRelativeTransform` (`self.RotationPivotComponent`)))
  (set `self.CachedTranslationPivotTransform` (`SceneComponent.GetRelativeTransform` (`self.TranslationPivotComponent`)))
  (bind _returnvalue (`SceneComponent.K2_AttachToComponent` (select `bool` (`local.L_Rotation`) :`false` (`self.TranslationPivotComponent`) :`true` (`self.RotationPivotComponent`)) (`local.L_Component`) "None" "SnapToTarget" "SnapToTarget" "SnapToTarget" false))
  (return _returnvalue))

(fn `DetachFromComponent`
  (returns (ReturnValue :type Boolean))
  (`SceneComponent.K2_DetachFromComponent` (`self.RotationPivotComponent`) "KeepRelative" "KeepRelative" "KeepRelative" true)
  (`SceneComponent.K2_DetachFromComponent` (`self.TranslationPivotComponent`) "KeepRelative" "KeepRelative" "KeepRelative" true)
  (`SceneComponent.K2_AttachToComponent` (`self.RotationPivotComponent`) (`self.RootComponent`) "None" "SnapToTarget" "SnapToTarget" "SnapToTarget" true)
  (`SceneComponent.K2_SetRelativeTransform` (`self.RotationPivotComponent`) (`self.CachedRotationPivotTransform`) false true)
  (`SceneComponent.K2_SetRelativeTransform` (`self.TranslationPivotComponent`) (`self.CachedTranslationPivotTransform`) false true)
  (`self.K2_SetActorTransform` (`KismetMathLibrary.MakeTransform` (0.0 0.0 -9999.0) (`self.K2_GetActorRotation`)))
  (return true))

(fn `GetComponentToAttach`
  (returns (Component :type "SceneComponent Object Reference"))
  (return (`self.SnapshotPivotComponent`)))

(fn `Rotate`
  (params (InRotation :type "Rotator Structure"))
  (returns (ReturnValue :type Boolean))
  (return false))

(fn `UserConstructionScript`)