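; Base collectible item that is resolved by touching sockets on its static mesh in a required order.
; Each touch maps to the closest socket within range, using the socket's X scale as its hit radius, and records the point and socket name.
; Once the recorded count matches SocketsOrder, an identical sequence marks the item resolved, while a mismatch clears the recorded touches.
; The reset event empties the required socket order.
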(event `WasTouched`
  (params (InLocation :type "Vector Structure"))
  (bind _returnvalue (`self.GetWasResolved`))
  (if (not _returnvalue)
    (bind _socket (`self.FindClosestSocket` InLocation))
    (if (!= _socket "None")
      (`KismetArrayLibrary.Array_Add` (`self.HittedPoints`) InLocation)
      (`KismetArrayLibrary.Array_Add` (`self.HittedSocketsOrder`) _socket)
      (if (== (`KismetArrayLibrary.Array_Length` (`self.HittedSocketsOrder`)) (`KismetArrayLibrary.Array_Length` (`self.SocketsOrder`)))
        (if (`KismetArrayLibrary.Array_Identical` (`self.HittedSocketsOrder`) (`self.SocketsOrder`))
          (`self.SetWasResolved` true)
          (else
            (set `self.HittedSocketsOrder` (`|MakeArray`))
            (set `self.HittedPoints` (`|MakeArray`))))))))

(event `Event_ResetItem`
  (set `self.SocketsOrder` (`|MakeArray`)))

(fn `FindClosestSocket`
  (params (HitLocation :type "Vector Structure"))
  (returns (Socket :type Name))
  (locals (L_HitLocation :type "Vector Structure") (NewLocalVar_0 :type Name :default "None") (L_SocketName :type Name) (L_PreviousSocketDistance :type "Float (double-precision)" :default 999999.0))
  (set `local.L_HitLocation` HitLocation)
  (for _array_element (`SceneComponent.GetAllSocketNames` (`self.StaticMeshComponent`))
    (bind _returnvalue (`KismetMathLibrary.VSize` (- (.location (`SceneComponent.GetSocketTransform` (`self.StaticMeshComponent`) _array_element "RTS_World")) (`local.L_HitLocation`))))
    (if (and (< _returnvalue (`local.L_PreviousSocketDistance`)) (< _returnvalue (.x (.scale (`SceneComponent.GetSocketTransform` (`self.StaticMeshComponent`) _array_element "RTS_World")))))
      (set `local.L_PreviousSocketDistance` _returnvalue)
      (set `local.L_SocketName` _array_element)))
  (return (`local.L_SocketName`)))

(fn `UserConstructionScript`
  (`parent.UserConstructionScript`))