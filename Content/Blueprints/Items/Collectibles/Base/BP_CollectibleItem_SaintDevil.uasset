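; Collectible item variant (Saint Devil) that turns part of its mesh a quarter turn when touched.
; A touch caches the part's relative rotation, calls the parent touch logic and plays a timeline that lerps SMRotatedPart to 90 degrees beyond that rotation.
; Touches are ignored while the timeline plays, so each later touch turns the part onward from where it stopped.
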(event `self.WasTouched`
  (params (InLocation :type "Vector Structure"))
  (if (not (`TimelineComponent.IsPlaying` (`self.Animation`)))
    (set `self.CachedRotation` (`SceneComponent.RelativeRotation` (`self.SM_RotatedPart`)))
    (`parent.WasTouched` InLocation)
    (bind (_direction _alpha) (`Timeline|Animation` :!via `PlayFromStart`)
      (:`Update`
        (`SceneComponent.K2_SetRelativeRotation` (`self.SM_RotatedPart`) (`KismetMathLibrary.RLerp` (`self.CachedRotation`) (`KismetMathLibrary.ComposeRotators` (`self.CachedRotation`) (struct :`Yaw` 90.0)) _alpha true) false false)))))

(fn `UserConstructionScript`
  (`parent.UserConstructionScript`))