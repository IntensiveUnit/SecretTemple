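; Collectible saint-and-devil statuette with two independently touchable parts that turn in quarter steps until the item is resolved.
; A touch locks input, caches the part's rotation and plays a timeline that lerps it 90 degrees in yaw, firing change-started and change-ended events.
; Top (Saint) and bottom (Devil) facings are read as enums from the socket closest to a reference socket.
; Construction shows numbered text labels only in debug.
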(event `self.WasTouched`
  (params (InLocation :type "Vector Structure") (InComponent :type "PrimitiveComponent Object Reference"))
  (bind _returnvalue (`self.GetWasResolved`))
  (if _returnvalue
    _
    (elif (or (== InComponent (`self.SM_RotatedPart_01`)) (== InComponent (`self.SM_RotatedPart_02`)))
      (if (not (`self.bIsLocked`))
        (set `self.bIsLocked` true)
        (set `self.CachedComponent` InComponent)
        (set `self.CachedRotation` (`SceneComponent.RelativeRotation` InComponent))
        (`self.OnItemChangeHasStarted` self self)
        (bind (_direction _alpha) (`Timeline|Animation` :!via `PlayFromStart`)
          (:`Update`
            (`SceneComponent.K2_SetRelativeRotation` (`self.CachedComponent`) (`KismetMathLibrary.RLerp` (`self.CachedRotation`) (`KismetMathLibrary.ComposeRotators` (`self.CachedRotation`) (struct :`Yaw` 90.0)) _alpha true) false false))
          (:`Finished`
            (switch `ETimelineDirection` _direction
              (:`Forward`
                (set `self.bIsLocked` false)
                (`self.OnItemChangeHasEnded` self self)))))))))

(fn `GetCurrentBottomSide`
  (returns (ReturnValue :type "/Game/Blueprints/Items/Collectibles/SaintAndDevilStatuette/E_Devil_Sockets Enum"))
  (bind _socket (`self.FindClosestSocket` (`SceneComponent.GetSocketLocation` (`self.StaticMeshComponent`) (`self.SocketName`)) (`self.SM_RotatedPart_01`)))
  (switch `name` _socket
    (:`Soc_Devil_01`
      (return "NewEnumerator4"))
    (:`Soc_Devil_02`
      (return "NewEnumerator5"))
    (:`Soc_Devil_03`
      (return "NewEnumerator6"))
    (:`Soc_Devil_04`
      (return "NewEnumerator7"))))

(fn `GetCurrentTopSide`
  (returns (ReturnValue :type "/Game/Blueprints/Items/Collectibles/SaintAndDevilStatuette/E_Saint_Sockets Enum"))
  (bind _socket (`self.FindClosestSocket` (`SceneComponent.GetSocketLocation` (`self.StaticMeshComponent`) (`self.SocketName`)) (`self.SM_RotatedPart_02`)))
  (switch `name` _socket
    (:`Soc_Saint_01`
      (return "NewEnumerator8"))
    (:`Soc_Saint_02`
      (return "NewEnumerator9"))
    (:`Soc_Saint_03`
      (return "NewEnumerator10"))
    (:`Soc_Saint_04`
      (return "NewEnumerator11"))))

(fn `UserConstructionScript`
  (`parent.UserConstructionScript`)
  (`SceneComponent.SetVisibility` (`self.Text_Number_08`) (`self.Debug`) false)
  (`SceneComponent.SetVisibility` (`self.Text_Number_07`) (`self.Debug`) false)
  (`SceneComponent.SetVisibility` (`self.Text_Number_06`) (`self.Debug`) false)
  (`SceneComponent.SetVisibility` (`self.Text_Number_01`) (`self.Debug`) false)
  (`SceneComponent.SetVisibility` (`self.Text_Number_02`) (`self.Debug`) false)
  (`SceneComponent.SetVisibility` (`self.Text_Number_03`) (`self.Debug`) false)
  (`SceneComponent.SetVisibility` (`self.Text_Number_04`) (`self.Debug`) false)
  (`SceneComponent.SetVisibility` (`self.Text_Number_05`) (`self.Debug`) false))