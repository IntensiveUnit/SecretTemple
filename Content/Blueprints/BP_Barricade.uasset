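; BP_Barricade is an interactable obstacle actor that is removed when a player or other instigator interacts with it.
; Interaction is always allowed, while using an item on it always returns false.
; Interacting spawns an emitter at the actor's transform, prints a placeholder message for an unfinished QTE, calls CallOnSuccessfully, then destroys the barricade.
; All logic lives in the interaction functions; the event graph and construction script are empty.
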(fn `CanInteractWithActor`
  (params (InteractionInstigator :type "PlayerCharacter Object Reference"))
  (returns (ReturnValue :type Boolean))
  (return true))

(fn `InteractWithActor`
  (params (InteractionInstigator :type "PlayerCharacter Object Reference"))
  (returns (ReturnValue :type Boolean))
  (`GameplayStatics.SpawnEmitterAtLocation` null (.location (`self.GetTransform`)) (.rotation (`self.GetTransform`)) (.scale (`self.GetTransform`)))
  (`KismetSystemLibrary.PrintString` "QTE EVENT UNDER DEVELOPMENT" true true (struct :`G` 0.66 :`B` 1.0 :`A` 1.0) 10.0)
  (`self.OnSuccessfully`)
  (`self.K2_DestroyActor`)
  (return true))

(fn `UseItemOnActor`
  (params (InteractionInstigator :type "PlayerCharacter Object Reference") (Item :type "Item Object Reference"))
  (returns (ReturnValue :type Boolean))
  (return false))

(fn `UserConstructionScript`)