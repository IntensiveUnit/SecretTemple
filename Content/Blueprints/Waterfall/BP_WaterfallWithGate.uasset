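; Waterfall actor with a gate, controlled by a lever that switches the waterfall off and back on.
; BeginPlay creates a dynamic material for the arc mesh and binds the lever's activate and deactivate attempts, paired with unrestricted response messages.
; One timeline fades the water's opacity and moves the gate between two transforms, reversing on deactivation as the sound fades to match.
; The construction script places the gate at its start transform.
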(event `self.ReceiveBeginPlay`
  (bind _returnvalue (`PrimitiveComponent.CreateDynamicMaterialInstance` (`self.SM_Waterfall_Arc`) 0 "/Game/Materials/Water/MIC_Waterfall_Arc.MIC_Waterfall_Arc" "None"))
  (set `self.MI_Waterfall` _returnvalue)
  (add `/Game/Blueprints/Lever/BP_Lever.OnTryToActivate` (`self.Lever`) (delegate `OnLeverTryActivate`))
  (add `/Game/Blueprints/Lever/BP_Lever.OnTryToDeactivate` (`self.Lever`) (delegate `OnLeverTryDeactivate`)))

(event `OnLeverTryActivate`
  (params (InLever :type "/Game/Blueprints/Lever/BP_Lever Object Reference")))

(event `OnLeverTryDeactivate`
  (params (InLever :type "/Game/Blueprints/Lever/BP_Lever Object Reference")))

(fn `UserConstructionScript`
  (`SceneComponent.K2_SetRelativeTransform` (`self.SM_Gateway`) (`self.StartAnimationTransform`) false false))