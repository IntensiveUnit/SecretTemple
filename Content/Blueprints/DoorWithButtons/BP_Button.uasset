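; BP_Button is an interactable toggle button that glows when pressed and signals its pressed and released states.
; Each interaction flips the Pressed flag, calls the matching OnWasPressed or OnWasReleased dispatcher, and plays the Animation timeline forward or in reverse.
; The timeline drives the Emissive parameter on a dynamic material created for the button mesh at BeginPlay.
; Interaction is blocked while the timeline plays, and using items on it is unsupported.
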(event `self.ReceiveBeginPlay`
  (bind _returnvalue (`PrimitiveComponent.CreateDynamicMaterialInstance` (`self.SM_ButtonMesh`) 0 (`PrimitiveComponent.GetMaterial` (`self.SM_ButtonMesh`) 0) "None"))
  (set `self.DMI_BodyMaterial` _returnvalue))

(event `Activate`
  (bind (_direction _animation) (`Timeline|Animation` :!via `PlayFromStart` :!label _label)
    (:`Update`
      (`MaterialInstanceDynamic.SetScalarParameterValue` (`self.DMI_BodyMaterial`) "Emissive" (* _animation 100.0)))))

(event `Deactivate`
  (goto _label :!via `ReverseFromEnd`))

(fn `CanInteractWithActor`
  (params (InteractionInstigator :type "PlayerCharacter Object Reference"))
  (returns (ReturnValue :type Boolean))
  (return (not (`TimelineComponent.IsPlaying` (`self.Animation`)))))

(fn `InteractWithActor`
  (params (InteractionInstigator :type "PlayerCharacter Object Reference"))
  (returns (ReturnValue :type Boolean))
  (if (`self.Pressed`)
    (set `self.Pressed` false)
    (`self.OnWasReleased` self)
    (`self.Deactivate`)
    (else
      (set `self.Pressed` true)
      (`self.OnWasPressed` self)
      (`self.Activate`)))
  (return true))

(fn `UseItemOnActor`
  (params (InteractionInstigator :type "PlayerCharacter Object Reference") (Item :type "Item Object Reference"))
  (returns (ReturnValue :type Boolean))
  (return false))

(fn `UserConstructionScript`)