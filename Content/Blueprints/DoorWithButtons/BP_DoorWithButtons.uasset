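; A puzzle door that slides open when its linked buttons are pressed in the correct order.
; The construction script takes ownership of the buttons in the expected sequence and binds their press and release events, which add to or remove from the current order.
; Once enough are pressed, a match plays a one-time timeline moving the door mesh, while a mismatch deactivates all buttons and clears the order, as does the animation finishing.
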(event `OnButtonPressed`
  (params (InButton :type "/Game/Blueprints/DoorWithButtons/BP_Button Object Reference"))
  (`KismetArrayLibrary.Array_Add` (`self.CurrentButtonOrder`) InButton)
  (if (>= (`KismetArrayLibrary.Array_Length` (`self.CurrentButtonOrder`)) (`KismetArrayLibrary.Array_Length` (`self.RightButtonOrder`)))
    (if (`KismetArrayLibrary.Array_Identical` (`self.CurrentButtonOrder`) (`self.RightButtonOrder`))
      (if (not (`self.WasOpened`))
        (set `self.WasOpened` true)
        (bind (_direction _animation) (`Timeline|Animation`)
          (:`Update`
            (`SceneComponent.K2_SetRelativeLocation` (`self.SM_Door`) (`KismetMathLibrary.VLerp` (.location (`self.StartAnimationTransform`)) (.location (`self.EndAnimationTransform`)) _animation) false false))
          (:`Finished`
            (for _array_element (`self.AllButtons`) :!label _label
              (`/Game/Blueprints/DoorWithButtons/BP_Button.Deactivate` _array_element))
            (`KismetArrayLibrary.Array_Clear` (`self.CurrentButtonOrder`)))))
      (else
        (goto _label)))))

(event `OnButtonReleased`
  (params (InButton :type "/Game/Blueprints/DoorWithButtons/BP_Button Object Reference"))
  (`KismetArrayLibrary.Array_RemoveItem` (`self.CurrentButtonOrder`) InButton))

(fn `UserConstructionScript`
  (for _array_element (`self.RightButtonOrder`)
    (`self.SetOwner` _array_element self)
    (bind _asbp_button (cast `/Game/Blueprints/DoorWithButtons/BP_Button` _array_element))
    (add `/Game/Blueprints/DoorWithButtons/BP_Button.OnWasPressed` _asbp_button (`|CreateDelegate` :!event `OnButtonPressed`))
    (add `/Game/Blueprints/DoorWithButtons/BP_Button.OnWasReleased` _asbp_button (`|CreateDelegate` :!event `OnButtonReleased`))))