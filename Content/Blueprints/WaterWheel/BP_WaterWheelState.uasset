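; BP_WaterWheelState is a skeleton state for the water wheel, with no gameplay behavior of its own.
; On BeginPlay it casts its owner to BP_WaterWheel, caches it and binds to that wheel's lever activated and deactivated events.
; Both lever handlers are empty, and the interact and use-item functions all return false, leaving neutral defaults for state-specific logic.
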(event `self.ReceiveBeginPlay`
  (bind _asbp_water_wheel (cast `/Game/Blueprints/WaterWheel/BP_WaterWheel` (`self.GetOwner`)))
  (set `self.WaterWheelOwner` _asbp_water_wheel)
  (add `/Game/Blueprints/Lever/BP_Lever.OnActivated` (`/Game/Blueprints/WaterWheel/BP_WaterWheel.Lever` (`self.WaterWheelOwner`)) (delegate `OnLeverActivated`))
  (add `/Game/Blueprints/Lever/BP_Lever.OnDeactivated` (`/Game/Blueprints/WaterWheel/BP_WaterWheel.Lever` (`self.WaterWheelOwner`)) (delegate `OnLeverDeactivated`)))

(event `OnLeverActivated`
  (params (InLever :type "/Game/Blueprints/Lever/BP_Lever Object Reference")))

(event `OnLeverDeactivated`
  (params (OnLever :type "/Game/Blueprints/Lever/BP_Lever Object Reference")))

(fn `CanInteractWithActor`
  (params (InteractionInstigator :type "PlayerCharacter Object Reference"))
  (returns (ReturnValue :type Boolean))
  (return false))

(fn `InteractWithActor`
  (params (InteractionInstigator :type "PlayerCharacter Object Reference"))
  (returns (ReturnValue :type Boolean))
  (return false))

(fn `UseItemOnActor`
  (params (InteractionInstigator :type "PlayerCharacter Object Reference") (Item :type "Item Object Reference"))
  (returns (ReturnValue :type Boolean))
  (return false))

(fn `UserConstructionScript`)