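; Sprint gameplay ability that makes the character sprint while the input is held, draining stamina over time.
; Activation starts sprinting on the CustomMovementComponent and waits for input release, which ends the ability.
; A one-second delay loop commits the ability cost only while accelerating and not falling, ending the ability when the commit fails.
; Ending the ability stops sprinting.
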(event `self.K2_ActivateAbility`
  (bind _l_movementcomponent (`self.L_MovementComponent`))
  (bind ((`MovementComponent` _movementcomponent)) (break `GameplayAbilityActorInfo` (`self.GetActorInfo`)))
  (`/Engine/EditorBlueprintResources/StandardMacros.IsValid` _movementcomponent
    (:`Is Valid`
      (bind _ascustom_movement_component (cast `CustomMovementComponent` _movementcomponent)
        (:`then`
          (bind _output_get (set `self.L_MovementComponent` _ascustom_movement_component))
          (`CustomMovementComponent.StartSprinting` _output_get)
          (bind _asynctaskproxy (`AbilityTask_WaitInputRelease.WaitInputRelease` false) ; If user release "Sprint" button end ability
            (:`then`
              (set `self.WaitInputRelease` _asynctaskproxy)
              (`AbilityTask_WaitDelay.WaitDelay` 1.0 :!label _label ; Draining stamina
                (:`OnFinish`
                  (if (and (> (`KismetMathLibrary.VSize` (`CharacterMovementComponent.GetCurrentAcceleration` _l_movementcomponent)) 0.0) (not (`NavMovementComponent.IsFalling` _l_movementcomponent)))
                    (bind _returnvalue (`self.K2_CommitAbilityCost` false)) ; Commit stamina cost
                    (if _returnvalue
                      (if (`KismetSystemLibrary.IsValid` (`self.WaitInputRelease`)) :!label _label_2
                        (goto _label))
                      (else
                        (`self.K2_EndAbility` :!label _label_3)))
                    (else
                      (goto _label_2))))))
            (:`OnRelease`
              (goto _label_3))))
        (:`CastFailed`
          (goto _label_3))))
    (:`Is Not Valid`
      (goto _label_3))))

(event `self.K2_OnEndAbility`
  (params (bWasCancelled :type Boolean))
  (`/Engine/EditorBlueprintResources/StandardMacros.IsValid` (`self.L_MovementComponent`)
    (:`Is Valid`
      (`CustomMovementComponent.StopSprinting` (`self.L_MovementComponent`)))))