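; Gameplay ability that lets the player character climb by switching it to Flying movement, reusing its walking braking deceleration.
; A per-tick loop applies the forward input scalar along the character's up vector.
; When the camera looks steeply downward, the direction becomes character-down blended with control-rotation forward.
; Ending the ability restores Walking mode; the file contains no climbable-surface detection.
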(event `self.K2_ActivateAbility`
  (bind _playercharacter (`self.PlayerCharacter`))
  (bind _charactermovement (`Character.CharacterMovement` (`self.PlayerCharacter`)))
  (`self.GetPlayerCharacter`)
  (`CharacterMovementComponent.SetMovementMode` (`Character.CharacterMovement` (`self.PlayerCharacter`)) "MOVE_Flying" 0)
  (set `CharacterMovementComponent.BrakingDecelerationFlying` (`CharacterMovementComponent.BrakingDecelerationWalking` _charactermovement) _charactermovement)
  (`KismetSystemLibrary.DelayUntilNextTick` :!label _label)
  (`Pawn.AddMovementInput` (`self.PlayerCharacter`) (* (`KismetMathLibrary.Normal` (`KismetMathLibrary.SelectVector` (`Actor.GetActorUpVector` _playercharacter) (+ (* (`Actor.GetActorUpVector` _playercharacter) (-1.0 -1.0 -1.0)) (`KismetMathLibrary.GetForwardVector` (`Pawn.GetControlRotation` _playercharacter))) (>= (`KismetMathLibrary.Dot_VectorVector` (`SceneComponent.GetForwardVector` (`PlayerCharacter.FollowCamera` (`self.PlayerCharacter`))) (`Actor.GetActorUpVector` (`self.PlayerCharacter`))) -0.5))) (`PlayerCharacter.GetMoveForwardInputScalar` (`self.PlayerCharacter`))) 1.0 false)
  (goto _label))

(event `self.K2_OnEndAbility`
  (params (bWasCancelled :type Boolean))
  (`self.PlayerCharacter`
    (:`then`
      _)
    (:`else`
      (`self.GetPlayerCharacter`)))
  (`CharacterMovementComponent.SetMovementMode` (`Character.CharacterMovement` (`self.PlayerCharacter`)) "MOVE_Walking" 0))

(fn `GetPlayerCharacter`
  (bind _asplayer_character (cast `PlayerCharacter` (`.AvatarActor` (break `GameplayAbilityActorInfo` (`self.GetActorInfo`)))))
  (set `self.PlayerCharacter` _asplayer_character))