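; Gameplay ability that toggles crouch on the owning Character.
; On activation it checks the movement component and avatar cast, caches the Character, crouches it and starts a WaitInputPress task.
; The next input press uncrouches and ends the ability, as does a failed validity check or cast.
; OnEndAbility also uncrouches the cached Character if valid, covering other ways the ability ends.
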(event `self.K2_ActivateAbility`
  (`/Engine/EditorBlueprintResources/StandardMacros.IsValid` (`.MovementComponent` (break `GameplayAbilityActorInfo` (`self.GetActorInfo`)))
    (:`Is Valid`
      (bind _ascharacter (cast `Character` (`.AvatarActor` (break `GameplayAbilityActorInfo` (`self.GetActorInfo`))))
        (:`then`
          (set `self.Character` _ascharacter)
          (bind _asynctaskproxy (`AbilityTask_WaitInputPress.WaitInputPress` false)
            (:`then`
              (set `self.WaitInputPress` _asynctaskproxy)
              (`Character.Crouch` (`self.Character`)))
            (:`OnPress`
              (`Character.UnCrouch` (`self.Character`) :!label _label)
              (`self.K2_EndAbility`))))
        (:`CastFailed`
          (goto _label))))
    (:`Is Not Valid`
      (goto _label))))

(event `self.K2_OnEndAbility`
  (params (bWasCancelled :type Boolean))
  (bind _character (`self.Character`)
    (:`then`
      (`Character.UnCrouch` _character))
    (:`else`)))