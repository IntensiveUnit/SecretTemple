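; Gameplay ability that makes the avatar jump along its facing direction using an ApplyRootMotionJumpForce task.
; Distance and height come from ability system attribute base values, chosen by whether the Character.Sprint tag is present.
; Distance drops to zero when the avatar has no velocity, giving a jump in place.
; The fixed-duration jump maintains its last root motion velocity, and the ability ends on finish or landing.
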(event `self.K2_ActivateAbility`
  (bind ((`AbilitySystemComponent` _abilitysystemcomponent)) (break `GameplayAbilityActorInfo` (`self.GetActorInfo`)))
  (bind ((`AvatarActor` _avataractor) (`AbilitySystemComponent` _abilitysystemcomponent_2)) (break `GameplayAbilityActorInfo` (`self.GetActorInfo`)))
  (bind _returnvalue (message `GameplayTagAssetInterface.HasMatchingGameplayTag` (`.AbilitySystemComponent` (break `GameplayAbilityActorInfo` (`self.GetActorInfo`))) (struct :`TagName` "Character.Sprint")))
  (set `self.L_HasSprintTag` _returnvalue)
  (`AbilityTask_ApplyRootMotionJumpForce.ApplyRootMotionJumpForce` "None" (`Actor.K2_GetActorRotation` (`.AvatarActor` (break `GameplayAbilityActorInfo` (`self.GetActorInfo`)))) (`KismetMathLibrary.SelectFloat` (`KismetMathLibrary.SelectFloat` (`.ReturnValue` (`AbilitySystemBlueprintLibrary.GetFloatAttributeBaseFromAbilitySystemComponent` _abilitysystemcomponent_2 (struct :`AttributeName` "WalkingJumpLength" :`Attribute` "/Script/SecretTemple.CustomAttributeSet:WalkingJumpLength" :`AttributeOwner` "Class'\"/Script/SecretTemple.CustomAttributeSet\"'"))) (`.ReturnValue` (`AbilitySystemBlueprintLibrary.GetFloatAttributeBaseFromAbilitySystemComponent` _abilitysystemcomponent_2 (struct :`AttributeName` "RunningJumpLength" :`Attribute` "/Script/SecretTemple.CustomAttributeSet:RunningJumpLength" :`AttributeOwner` "Class'\"/Script/SecretTemple.CustomAttributeSet\"'"))) (`self.L_HasSprintTag`)) 0.0 (> (`KismetMathLibrary.VSize` (`Actor.GetVelocity` _avataractor)) 0.0)) (`KismetMathLibrary.SelectFloat` (`.ReturnValue` (`AbilitySystemBlueprintLibrary.GetFloatAttributeBaseFromAbilitySystemComponent` _abilitysystemcomponent (struct :`AttributeName` "WalkingJumpHeight" :`Attribute` "/Script/SecretTemple.CustomAttributeSet:WalkingJumpHeight" :`AttributeOwner` "Class'\"/Script/SecretTemple.CustomAttributeSet\"'"))) (`.ReturnValue` (`AbilitySystemBlueprintLibrary.GetFloatAttributeBaseFromAbilitySystemComponent` _abilitysystemcomponent (struct :`AttributeName` "RunningJumpHeight" :`Attribute` "/Script/SecretTemple.CustomAttributeSet:RunningJumpHeight" :`AttributeOwner` "Class'\"/Script/SecretTemple.CustomAttributeSet\"'"))) (`self.L_HasSprintTag`)) 0.75 0.75 false "MaintainLastRootMotionVelocity"
    (:`OnFinish`
      _)
    (:`OnLanded`
      _))
  (`self.K2_EndAbility`))