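; Water wheel puzzle actor that spins a pivot and fades watermill sound in while its lever is active.
; It answers the lever's activation attempts with whether the Gateway was opened, and always allows deactivation.
; Lever events start or stop the rotation timeline and sound.
; Separate helpers spawn state actors per WaterWheelState but are unused by the event graph, and interaction functions return false.
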(event `self.ReceiveBeginPlay`
  (`AudioComponent.FadeOut` (`self.S_Watermill`) 0.0 0.0 "Linear")
  (add `/Game/Puzzle_Waterfall/Lever/BP_Lever.OnTryToActivate` (`self.Lever`) (delegate `OnLeverTryActivate`))
  (add `/Game/Puzzle_Waterfall/Lever/BP_Lever.OnTryToDeactivate` (`self.Lever`) (delegate `OnLeverTryDeactivate`))
  (add `/Game/Puzzle_Waterfall/Lever/BP_Lever.OnActivated` (`self.Lever`) (delegate `OnLeverActivated`))
  (add `/Game/Puzzle_Waterfall/Lever/BP_Lever.OnDeactivated` (`self.Lever`) (delegate `OnLeverDeactivated`)))

(event `OnLeverActivated`
  (params (InLever :type "/Game/Puzzle_Waterfall/Lever/BP_Lever Object Reference"))
  (set `self.bIsActivated` true)
  (`AudioComponent.FadeIn` (`self.S_Watermill`) 3.0 1.0 0.0 "Linear")
  (bind (_direction _animation) (`Timeline|Animation` :!label _label)
    (:`Update`
      (`SceneComponent.K2_SetRelativeRotation` (`self.SC_Pivot`) (`KismetMathLibrary.RLerp` (struct) (struct :`Pitch` 360.0) _animation) false false))))

(event `OnLeverTryActivate`
  (params (InLever :type "/Game/Puzzle_Waterfall/Lever/BP_Lever Object Reference"))
  (`InteractInterface.TakeResponseFromActor` InLever self (`/Game/Puzzle_Waterfall/BP_Gateway.bWasOpened` (`self.Gateway`))))

(event `OnLeverTryDeactivate`
  (params (InLever :type "/Game/Puzzle_Waterfall/Lever/BP_Lever Object Reference"))
  (`InteractInterface.TakeResponseFromActor` InLever self true))

(event `OnLeverDeactivated`
  (params (OnLever :type "/Game/Puzzle_Waterfall/Lever/BP_Lever Object Reference"))
  (set `self.bIsActivated` false)
  (`AudioComponent.FadeOut` (`self.S_Watermill`) 3.0 0.0 "Linear")
  (goto _label :!via `Stop`))

(fn `CanInteractWithActor`
  (params (InteractionInstigator :type "PlayerCharacter Object Reference"))
  (returns (ReturnValue :type Boolean))
  (return false))

(fn `DestroyCurrentState`
  (`/Engine/EditorBlueprintResources/StandardMacros.IsValid` (`self.CurrentState`)
    (:`Is Valid`
      (`self.K2_DestroyActor` (`self.CurrentState`)))
    (:`Is Not Valid`
      _))
  (return))

(fn `GetCurrentState`
  (returns (CurrentState :type "/Game/Puzzle_Waterfall/WaterWheel/BP_WaterWheelState Object Reference"))
  (`/Engine/EditorBlueprintResources/StandardMacros.IsValid` (`self.CurrentState`)
    (:`Is Valid`
      (return (`self.CurrentState`)))
    (:`Is Not Valid`
      (`self.InitializeState`)
      (return (`self.CurrentState`)))))

(fn `InitializeState`
  (switch `/Game/Puzzle_Waterfall/WaterWheel/E_WaterWheelState` (`self.WaterWheelState`)
    (:`NewEnumerator0`
      (bind _returnvalue (`|SpawnActorFromClass` "/Game/Puzzle_Waterfall/WaterWheel/BP_WaterWheelState_Activated.BP_WaterWheelState_Activated_C" (`self.GetTransform`) "Undefined" "OverrideRootScale" self null))
      (set `self.CurrentState` _returnvalue))
    (:`NewEnumerator1`
      (bind _returnvalue_2 (`|SpawnActorFromClass` "/Game/Puzzle_Waterfall/WaterWheel/BP_WaterWheelState_Deactivated.BP_WaterWheelState_Deactivated_C" (`self.GetTransform`) "Undefined" "OverrideRootScale" self null))
      (set `self.CurrentState` _returnvalue_2))
    (:`NewEnumerator2`
      (bind _returnvalue_3 (`|SpawnActorFromClass` "/Game/Puzzle_Waterfall/WaterWheel/BP_WaterWheelState_Deactivated.BP_WaterWheelState_Deactivated_C" (`self.GetTransform`) "Undefined" "OverrideRootScale" self null))
      (set `self.CurrentState` _returnvalue_3)))
  (return))

(fn `InteractWithActor`
  (params (InteractionInstigator :type "PlayerCharacter Object Reference"))
  (returns (ReturnValue :type Boolean))
  (return false))

(fn `SetCurrentState`
  (params (WaterWheelState :type "/Game/Puzzle_Waterfall/WaterWheel/E_WaterWheelState Enum" :default "NewEnumerator0"))
  (locals (L_NewState :type "/Game/Puzzle_Waterfall/WaterWheel/E_WaterWheelState Enum"))
  (set `local.L_NewState` WaterWheelState)
  (if (`|EnumInequality` (`local.L_NewState`) (`self.WaterWheelState`))
    (set `self.WaterWheelState` (`local.L_NewState`))
    (`self.DestroyCurrentState`)
    (`self.InitializeState`)
    (else
      (return))))

(fn `TakeResponseFromActor`
  (params (ResponseInstigator :type "Actor Object Reference") (bResponse :type Boolean))
  (returns (ReturnValue :type Boolean))
  (return false))

(fn `UseItemOnActor`
  (params (InteractionInstigator :type "PlayerCharacter Object Reference") (Item :type "Item Object Reference"))
  (returns (ReturnValue :type Boolean))
  (return false))

(fn `UserConstructionScript`)