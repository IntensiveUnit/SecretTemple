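; State actor for the activated water wheel in the waterfall puzzle, reacting to lever events through its WaterWheelOwner reference.
; On lever activation, it fades in the watermill sound and plays a timeline that lerps the wheel pivot through a full rotation.
; Deactivation cuts the sound and stops the timeline.
; Both events send a false response back to the owner's lever.
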(event `self.OnLeverActivated`
  (`InteractInterface.TakeResponseFromActor` (`/Game/Puzzle_Waterfall/WaterWheel/BP_WaterWheel.Lever` (`self.WaterWheelOwner`)) self false)
  (`AudioComponent.FadeIn` (`/Game/Puzzle_Waterfall/WaterWheel/BP_WaterWheel.S_Watermill` (`self.WaterWheelOwner`)) 3.0 1.0 0.0 "Linear")
  (bind (_direction _animation) (`Timeline|WaterWheelAnimation` :!label _label)
    (:`Update`
      (`SceneComponent.K2_SetRelativeRotation` (`/Game/Puzzle_Waterfall/WaterWheel/BP_WaterWheel.SC_Pivot` (`self.WaterWheelOwner`)) (`KismetMathLibrary.RLerp` (struct) (struct :`Pitch` 360.0) _animation) false false))))

(event `self.OnLeverDeactivated`
  (`InteractInterface.TakeResponseFromActor` (`/Game/Puzzle_Waterfall/WaterWheel/BP_WaterWheel.Lever` (`self.WaterWheelOwner`)) self false)
  (`AudioComponent.FadeOut` (`/Game/Puzzle_Waterfall/WaterWheel/BP_WaterWheel.S_Watermill` (`self.WaterWheelOwner`)) 0.0 0.0 "Linear")
  (goto _label :!via `Stop`))

(fn `UserConstructionScript`
  (`parent.UserConstructionScript`))