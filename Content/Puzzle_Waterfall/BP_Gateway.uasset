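; Waterfall puzzle gateway whose two gate meshes are opened and closed by a linked lever, once any linked barricade is destroyed.
; Binds to barricade and lever events, answering each lever attempt with CanBeOpened and, if allowed, playing or reversing the OpenGateWay timeline.
; The timeline is meant to lerp both gates between configurable start and end transforms, with start poses applied in the construction script.
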(event `self.ReceiveBeginPlay`
  (set `self.CanBeOpened` (not (`KismetSystemLibrary.IsValid` (`self.Barricade`))))
  (`|ExecutionSequence`
    (:`then_0`
      (bind _barricade (`self.Barricade`)
        (:`then`
          (add `/Game/Puzzle_Waterfall/BP_Barricade.OnSuccessfully` _barricade (delegate `OnBarricadeDestroyed`)))
        (:`else`)))
    (:`then_1`
      (bind _lever (`self.Lever`)
        (:`then`
          (add `/Game/Puzzle_Waterfall/Lever/BP_Lever.OnTryToActivate` _lever (delegate `OnLeverTryActivate`))
          (add `/Game/Puzzle_Waterfall/Lever/BP_Lever.OnTryToDeactivate` _lever (delegate `OnLeverTryDeactivate`)))
        (:`else`)))))

(event `OnBarricadeDestroyed`
  (set `self.CanBeOpened` true))

(event `OnLeverTryActivate`
  (params (InLever :type "/Game/Puzzle_Waterfall/Lever/BP_Lever Object Reference"))
  (`InteractInterface.TakeResponseFromActor` InLever self (`self.CanBeOpened`))
  (if (`self.CanBeOpened`)
    (`TimelineComponent.Play` (`self.OpenGateWay`))
    (set `self.bWasOpened` true)))

(event `OnLeverTryDeactivate`
  (params (InLever :type "/Game/Puzzle_Waterfall/Lever/BP_Lever Object Reference"))
  (`InteractInterface.TakeResponseFromActor` InLever self (`self.CanBeOpened`))
  (if (`self.CanBeOpened`)
    (`TimelineComponent.Reverse` (`self.OpenGateWay`))
    (set `self.bWasOpened` false)))

(fn `CanInteractWithActor`
  (params (InteractionInstigator :type "PlayerCharacter Object Reference"))
  (returns (ReturnValue :type Boolean))
  (return (and (`self.CanBeOpened`) (not (`TimelineComponent.IsPlaying` (`self.OpenGateWay`))))))

(fn `InteractWithActor`
  (params (InteractionInstigator :type "PlayerCharacter Object Reference"))
  (returns (ReturnValue :type Boolean)))

(fn `TakeResponseFromActor`
  (params (ResponseInstigator :type "Actor Object Reference") (bResponse :type Boolean))
  (returns (ReturnValue :type Boolean))
  (return false))

(fn `UseItemOnActor`
  (params (InteractionInstigator :type "PlayerCharacter Object Reference") (Item :type "Item Object Reference"))
  (returns (ReturnValue :type Boolean))
  (return false))

(fn `UserConstructionScript`
  (`SceneComponent.K2_SetRelativeTransform` (`self.SM_Gate_01`) (`self.FirstGateStartTransform`) false false)
  (`SceneComponent.K2_SetRelativeTransform` (`self.SM_Gate_02`) (`self.SecondGateStartTransform`) false false))