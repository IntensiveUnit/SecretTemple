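; Water plane for the waterfall puzzle that lowers when a linked lever activates and rises when one deactivates.
; On BeginPlay it binds to the activate and deactivate events of every entry in Levers.
; Each event caches the pivot's current relative transform and restarts a timeline that lerps it a fixed vertical step.
; Steps are relative to the position at trigger time, so an event arriving mid-animation starts from that intermediate height.
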(event `self.ReceiveBeginPlay`
  (for _array_element (`self.Levers`)
    (add `/Game/Puzzle_Waterfall/Lever/BP_Lever.OnActivated` _array_element (delegate `OnLeverActivated`))
    (add `/Game/Puzzle_Waterfall/Lever/BP_Lever.OnDeactivated` _array_element (delegate `OnLeverDeactivated`))))

(event `OnLeverActivated`
  (params (InLever :type "/Game/Puzzle_Waterfall/Lever/BP_Lever Object Reference"))
  (`self.PlayAnimationDown` true))

(event `OnLeverDeactivated`
  (params (OnLever :type "/Game/Puzzle_Waterfall/Lever/BP_Lever Object Reference"))
  (`self.PlayAnimationDown` false))

(event `PlayAnimationDown`
  (params (`Down/Up` :type Boolean))
  (set `self.CachedRelativeTransform` (`SceneComponent.GetRelativeTransform` (`self.SC_Pivot`)))
  (bind (_direction _alpha) (`Timeline|Animation` :!via `PlayFromStart`)
    (:`Update`
      (`SceneComponent.K2_SetRelativeLocation` (`self.SC_Pivot`) (`KismetMathLibrary.VLerp` (.location (`self.CachedRelativeTransform`)) (- (.location (`self.CachedRelativeTransform`)) (`KismetMathLibrary.SelectVector` (0.0 0.0 125.0) (0.0 0.0 -125.0) `Down/Up`)) _alpha) false false))))

(fn `UserConstructionScript`)