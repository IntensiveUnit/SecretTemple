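; Interactable lever for the waterfall puzzle that exists either with or without its handle, using the State pattern.
; It spawns a state actor matching WaterfallPultState on BeginPlay and destroys it on state change or its own destruction.
; Interaction, item-use and response calls are delegated to that state actor.
; The construction script only toggles handle mesh visibility, because states cannot be spawned there.
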(event `self.ReceiveBeginPlay`
  (`self.InitializeState`))

(event `self.ReceiveDestroyed`
  (`self.DestroyCurrentState`))

(fn `CanInteractWithActor`
  (params (InteractionInstigator :type "PlayerCharacter Object Reference"))
  (returns (ReturnValue :type Boolean))
  (bind _currentstate (`self.GetCurrentState`))
  (bind _returnvalue (`InteractInterface.CanInteractWithActor` _currentstate InteractionInstigator))
  (return _returnvalue))

(fn `DestroyCurrentState`
  (`/Engine/EditorBlueprintResources/StandardMacros.IsValid` (`self.CurrentState`)
    (:`Is Valid`
      (`self.K2_DestroyActor` (`self.CurrentState`)))
    (:`Is Not Valid`
      _))
  (return))

(fn `GetCurrentState`
  (returns (CurrentState :type "/Game/Puzzle_Waterfall/Lever/BP_LeverState Object Reference"))
  (`/Engine/EditorBlueprintResources/StandardMacros.IsValid` (`self.CurrentState`)
    (:`Is Valid`
      (return (`self.CurrentState`)))
    (:`Is Not Valid`
      (`self.InitializeState`)
      (return (`self.CurrentState`)))))

(fn `InitializeState`
  (switch `/Game/Puzzle_Waterfall/Lever/E_LeverStates` (`self.WaterfallPultState`)
    (:`NewEnumerator0`
      (bind _returnvalue (`|SpawnActorFromClass` "/Game/Puzzle_Waterfall/Lever/BP_LeverState_WithoutHandle.BP_LeverState_WithoutHandle_C" (`self.GetTransform`) "Undefined" "OverrideRootScale" self null))
      (set `self.CurrentState` _returnvalue)
      (return))
    (:`NewEnumerator1`
      (bind _returnvalue_2 (`|SpawnActorFromClass` "/Game/Puzzle_Waterfall/Lever/BP_LeverState_WithHandle.BP_LeverState_WithHandle_C" (`self.GetTransform`) "Undefined" "OverrideRootScale" self null))
      (set `self.CurrentState` _returnvalue_2)
      (return))))

(fn `InteractWithActor`
  (params (InteractionInstigator :type "PlayerCharacter Object Reference"))
  (returns (ReturnValue :type Boolean))
  (bind _currentstate (`self.GetCurrentState`))
  (bind _returnvalue (`InteractInterface.InteractWithActor` _currentstate InteractionInstigator))
  (return _returnvalue))

(fn `SetCurrentState`
  (params (WaterfallPultState :type "/Game/Puzzle_Waterfall/Lever/E_LeverStates Enum" :default "NewEnumerator0"))
  (locals (L_NewState :type "/Game/Puzzle_Waterfall/Lever/E_LeverStates Enum" :default "NewEnumerator0"))
  (set `local.L_NewState` WaterfallPultState)
  (if (`|EnumInequality` (`local.L_NewState`) (`self.WaterfallPultState`))
    (set `self.WaterfallPultState` (`local.L_NewState`))
    (`self.DestroyCurrentState`)
    (`self.InitializeState`)
    (else
      (return))))

(fn `TakeResponseFromActor`
  (params (ResponseInstigator :type "Actor Object Reference") (bResponse :type Boolean))
  (returns (ReturnValue :type Boolean))
  (bind _returnvalue (`InteractInterface.TakeResponseFromActor` (`self.CurrentState`) ResponseInstigator bResponse))
  (return _returnvalue))

(fn `UseItemOnActor`
  (params (InteractionInstigator :type "PlayerCharacter Object Reference") (Item :type "Item Object Reference"))
  (returns (ReturnValue :type Boolean))
  (bind _currentstate (`self.GetCurrentState`))
  (bind _returnvalue (`InteractInterface.UseItemOnActor` _currentstate InteractionInstigator Item))
  (return _returnvalue))

(fn `UserConstructionScript`
  ;[1 1 1] A crutch because you can't spawn a state in construction script
  (switch `/Game/Puzzle_Waterfall/Lever/E_LeverStates` (`self.WaterfallPultState`)
    (:`NewEnumerator0`
      (`SceneComponent.SetVisibility` (`self.SM_Handle`) false false))
    (:`NewEnumerator1`
      (`SceneComponent.SetVisibility` (`self.SM_Handle`) true false))))