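; Waterfall puzzle actor whose linked lever moves a gateway mesh and fades the waterfall out or back in.
; Binds to the lever's try-activate and try-deactivate events, always answering positively so the actor never blocks it.
; One timeline, played or reversed, drives the arc's dynamic material opacity and lerps the gate between start and end transforms, alongside the sound fade.
; The construction script places the gate at its start transform.
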(event `self.ReceiveBeginPlay`
  (bind _returnvalue (`PrimitiveComponent.CreateDynamicMaterialInstance` (`self.SM_Waterfall_Arc`) 0 "/Game/WaterMaterials/Materials/MIC_Waterfall_Arc.MIC_Waterfall_Arc" "None"))
  (set `self.MI_Waterfall` _returnvalue)
  (add `/Game/Puzzle_Waterfall/Lever/BP_Lever.OnTryToActivate` (`self.Lever`) (delegate `OnLeverTryActivate`))
  (add `/Game/Puzzle_Waterfall/Lever/BP_Lever.OnTryToDeactivate` (`self.Lever`) (delegate `OnLeverTryDeactivate`)))

(event `OnLeverTryActivate`
  (params (InLever :type "/Game/Puzzle_Waterfall/Lever/BP_Lever Object Reference"))
  ;[1 1 1] Positive response means this actor has no restrictions to be activated
  (message `InteractInterface.TakeResponseFromActor` InLever self true)
  (`AudioComponent.FadeOut` (`self.S_Waterfall`) 3.0 0.0 "Linear")
  (bind (_direction _alpha) (`Timeline|Waterfall animation` :!label _label)
    (:`Update`
      (`MaterialInstanceDynamic.SetScalarParameterValue` (`self.MI_Waterfall`) "Opacity" (`KismetMathLibrary.Lerp` 0.25 0.0 _alpha))
      (`SceneComponent.K2_SetRelativeLocationAndRotation` (`self.SM_Gateway`) (`KismetMathLibrary.VLerp` (.location (`self.StartAnimationTransform`)) (.location (`self.EndAnimationTransform`)) _alpha) (`KismetMathLibrary.RLerp` (.rotation (`self.StartAnimationTransform`)) (.rotation (`self.EndAnimationTransform`)) _alpha) false false))))

(event `OnLeverTryDeactivate`
  (params (InLever :type "/Game/Puzzle_Waterfall/Lever/BP_Lever Object Reference"))
  (message `InteractInterface.TakeResponseFromActor` InLever self true)
  (`AudioComponent.FadeIn` (`self.S_Waterfall`) 3.0 1.0 0.0 "Linear")
  (goto _label :!via `Reverse`))

(fn `UserConstructionScript`
  (`SceneComponent.K2_SetRelativeTransform` (`self.SM_Gateway`) (`self.StartAnimationTransform`) false false))